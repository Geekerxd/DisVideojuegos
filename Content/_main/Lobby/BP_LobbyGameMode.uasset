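; Lobby game mode for a multiplayer session that tracks joined players, host-selected map settings and character choices before launching the match.
; PostLogin initializes each player's lobby controller from Steam game instance settings, and EveryoneUpdate pushes roster, available characters and kick list while checking start readiness.
; Controllers are reached through interface messages for settings updates, kicks and loading screens.
; Character changes respawn and possess pawns at a PlayerStart, and launch server-travels by map ID.
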(event `self.K2_PostLogin`
  (params (NewPlayer :type "PlayerController Object Reference"))
  (bind _output_get (set `self.ConnectedPlayer` NewPlayer))
  (`KismetArrayLibrary.Array_AddUnique` (`self.ConnectedPlayers`) _output_get)
  (bind _outactors (`GameplayStatics.GetAllActorsOfClass` "/Script/Engine.PlayerStart"))
  (set `self.SpawnPoints` _outactors)
  (bind _gameinstance (message `/Game/_main/BPI_GameInstance.SteamGameInstanceRef` (`GameplayStatics.GetGameInstance`)))
  (set `self.Server Name` (`/Game/_main/SteamGameInstance.Server Name` _gameinstance))
  (set `self.Max Players` (`/Game/_main/SteamGameInstance.Max Players` _gameinstance))
  (bind _newparam (message `/Game/_main/Lobby/BPI_LobbyPC.LobbyPCRef` (`self.ConnectedPlayer`)))
  (bind _output_get_2 (set `self.LobbyPC` _newparam))
  (`/Game/_main/Lobby/BP_LobbyPC.initialSetup` _output_get_2 (`self.Server Name`) (`self.SelectedMapImage`) (`self.SelectedMapName`) (`self.SelectedMapTime`)))

(event `SpawnPlayer`
  (params (Player :type "PlayerController Object Reference")))

(event `EveryoneUpdate`
  (bind _connectedplayers (`self.ConnectedPlayers`))
  (bind _output_get (set `self.CurrentPlayers` (`KismetArrayLibrary.Array_Length` (`self.ConnectedPlayers`))))
  (if (> _output_get 0)
    (`KismetArrayLibrary.Array_Clear` (`self.ConnectedPlayersInfo`))
    (for _array_element _connectedplayers
      (bind _newparam (message `/Game/_main/Lobby/BPI_LobbyPC.LobbyPCRef` _array_element))
      (`KismetArrayLibrary.Array_AddUnique` (`self.ConnectedPlayersInfo`) (`/Game/_main/Lobby/BP_LobbyPC.PlayerSettings` _newparam))
      (`/Game/_main/Lobby/BP_LobbyPC.UpdateNumPlayers` _newparam (`self.CurrentPlayers`) (`self.Max Players`)))
    (for _array_element_2 _connectedplayers
      (bind _newparam_2 (message `/Game/_main/Lobby/BPI_LobbyPC.LobbyPCRef` _array_element_2))
      (`/Game/_main/Lobby/BP_LobbyPC.AddPlayerInfo` _newparam_2 (`self.ConnectedPlayersInfo`))
      (`/Game/_main/Lobby/BP_LobbyPC.UpdateAviableCharacters` _newparam_2 (`self.Availablecharacters`))
      (`self.AddToKickList`))
    (for _array_element_3 (`self.ConnectedPlayersInfo`) :!label _label
      (if (== (`.PlayerCharacter_16_63F8F8394FBEEE06F3BAFA8F704F63F0` (break `/Game/_main/S_PlayerInfo` _array_element_3)) null)
        (set `self.CanWeStart?` false)
        (`self.Cannotstartgame`)
        (else
          (set `self.CanWeStart?` true))))))

(event `Cannotstartgame`
  (goto _label :!via `Break`))

(event `HostUpdateSetting`
  (params (SelectedMapImage :type "Texture2D Object Reference") (SelectedMapName :type Text) (SelectedMapTime :type Text) (selectedMapId :type Integer))
  (set `self.SelectedMapImage` SelectedMapImage)
  (set `self.SelectedMapName` SelectedMapName)
  (set `self.SelectedMapTime` SelectedMapTime)
  (set `self.selectedMapId` selectedMapId)
  (for _array_element (`self.ConnectedPlayers`)
    (bind _newparam (message `/Game/_main/Lobby/BPI_LobbyPC.LobbyPCRef` _array_element))
    (`/Game/_main/Lobby/BP_LobbyPC.UpdateLobbySettings` _newparam (`self.SelectedMapImage`) (`self.SelectedMapName`) (`self.SelectedMapTime`))))

(event `PlayerKicked`
  (params (PLayerID :type Integer))
  ;[1 1 1] kickea a jugador de session
  (bind _newparam (message `/Game/_main/Lobby/BPI_LobbyPC.LobbyPCRef` (`|GetArrayItem` (`self.ConnectedPlayers`) PLayerID)))
  (`/Game/_main/Lobby/BP_LobbyPC.kicked` _newparam))

(event `AddToKickList`
  (bind _newparam (message `/Game/_main/Lobby/BPI_LobbyPC.LobbyPCRef` (`GameplayStatics.GetPlayerController` 0)))
  (`/Game/_main/Lobby/BP_LobbyPC.AddPlayerToKickWindow` _newparam))

(event `self.K2_OnLogout`
  (params (ExitingController :type "Controller Object Reference"))
  (bind _connectedplayers (`self.ConnectedPlayers`))
  (for (_array_element _array_index) _connectedplayers
    (if (== _array_element ExitingController)
      (break)))
  (bind _newparam (message `/Game/_main/Lobby/BPI_LobbyPC.LobbyPCRef` (`|GetArrayItem` _connectedplayers _array_index)))
  (`KismetArrayLibrary.Array_Set` (`self.Availablecharacters`) (`/Game/_main/Lobby/BP_LobbyPC.SelectedCharacter` _newparam))
  (`KismetArrayLibrary.Array_Remove` (`self.ConnectedPlayers`) _array_index)
  (`KismetArrayLibrary.Array_Remove` (`self.ConnectedPlayersInfo`) _array_index)
  (`self.EveryoneUpdate`))

(event `StartLoadingScreen`
  ;[1 1 1] muestra pantalla de carga y corre el juego
  (for _array_element (`self.ConnectedPlayers`)
    (bind _newparam (message `/Game/_main/Lobby/BPI_LobbyPC.LobbyPCRef` _array_element))
    (`/Game/_main/Lobby/BP_LobbyPC.ShowLoadingScreen` _newparam))
  (`self.LaunchGame`))

(event `LaunchGame`
  ;[1 1 1] muestra pantalla de carga y corre el juego
  (switch `int` (`self.selectedMapId`)
    (:`0`
      (`KismetSystemLibrary.ExecuteConsoleCommand` "servertravel/Game/FirstPersonBP/Maps/FirstPersonExampleMap" (`GameplayStatics.GetPlayerController` 0)))))

(event `ChangeCharacter`
  (params (ConnectedPlayer :type "PlayerController Object Reference") (CharacterClass :type "Character Class Reference") (ChangedStatus :type Boolean))
  (bind _spawnpoints (`self.SpawnPoints`))
  ;[1 1 1] spawn el personaje elegido
  (if (not ChangedStatus)
    (`/Engine/EditorBlueprintResources/StandardMacros.IsValid` (`Controller.K2_GetPawn` ConnectedPlayer)
      (:`Is Valid`
        (`self.K2_DestroyActor`))
      (:`Is Not Valid`
        _))
    (bind _returnvalue (`|SpawnActorFromClass` CharacterClass (`self.GetTransform` (`|GetArrayItem` _spawnpoints (- (`KismetArrayLibrary.Array_Length` _spawnpoints) 1))) "AlwaysSpawn" "OverrideRootScale" null null))
    (`Controller.Possess` ConnectedPlayer _returnvalue)))

(fn `LobbyGMref`
  (returns (LobbyGM :type "/Game/_main/Lobby/BP_LobbyGameMode Object Reference"))
  (return self))

(fn `UserConstructionScript`)