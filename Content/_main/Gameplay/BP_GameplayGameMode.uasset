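; Multiplayer gameplay game mode that tracks player controllers, spawns their selected characters and relays chat.
; BeginPlay caches all PlayerStarts, and SpawnPlayer spawns and possesses the character at a random one when the controller has no valid pawn.
; Controllers registered in OnSwapPlayerControllers receive every chat message.
; Logout asks the Steam game instance to destroy the exiting controller's session, using interface-style reference messages.
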(event `self.K2_OnSwapPlayerControllers`
  (params (OldPC :type "PlayerController Object Reference") (NewPC :type "PlayerController Object Reference"))
  (`KismetArrayLibrary.Array_Add` (`self.AllPlayersControllers`) NewPC))

(event `self.ReceiveBeginPlay`
  (bind _outactors (`GameplayStatics.GetAllActorsOfClass` "/Script/Engine.PlayerStart"))
  (set `self.SpawnPoints` _outactors))

(event `SpawnPlayer`
  (params (playercontroller :type "PlayerController Object Reference") (SelectedCharacter :type "Character Class Reference"))
  (bind _spawnpoints (`self.SpawnPoints`))
  ;[1 1 1] Spawn the player at a random place
  (`/Engine/EditorBlueprintResources/StandardMacros.IsValid` (`Controller.K2_GetPawn` playercontroller)
    (:`Is Valid`
      (`self.K2_DestroyActor`))
    (:`Is Not Valid`
      (bind _returnvalue (`|SpawnActorFromClass` SelectedCharacter (`self.GetTransform` (`|GetArrayItem` _spawnpoints (`KismetMathLibrary.RandomIntegerInRange` 0 (- (`KismetArrayLibrary.Array_Length` _spawnpoints) 1)))) "AlwaysSpawn" "OverrideRootScale" null null))
      (`Controller.Possess` playercontroller _returnvalue))))

(event `self.K2_OnLogout`
  (params (ExitingController :type "Controller Object Reference"))
  (bind _gampleypc (message `/Game/_main/Gameplay/BPI_GameplayPC.GameplayPCRef` ExitingController))
  (bind _gameinstance (message `/Game/_main/BPI_GameInstance.SteamGameInstanceRef` (`GameplayStatics.GetGameInstance`)))
  (message `/Game/_main/BPI_GameInstance.DestroySessionCaller` _gameinstance _gampleypc))

(event `UpdateChat`
  (params (Sender :type Text) (ChatText :type Text))
  (for _array_element (`self.AllPlayersControllers`)
    (bind _gampleypc (message `/Game/_main/Gameplay/BPI_GameplayPC.GameplayPCRef` _array_element))
    (`/Game/_main/Gameplay/BP_GameplayPC.UpdateChatWindow` _gampleypc Sender ChatText)))

(fn `GameplayGMRef`
  (returns (GameplayGMref :type "/Game/_main/Gameplay/BP_GameplayGameMode Object Reference"))
  (return self))

(fn `UserConstructionScript`)