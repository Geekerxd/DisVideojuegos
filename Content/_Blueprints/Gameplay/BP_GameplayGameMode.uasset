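; Gameplay game mode for a Steam multiplayer session that handles character spawning, chat and player logout.
; SpawnPlayer spawns the selected character at a random PlayerStart and has the controller possess it.
; Controllers are collected on swap into AllPlayerControllers, which UpdateChat loops over to push each message to every chat window.
; Reference-getter messages link game mode, controllers and Steam game instance, which destroys the exiting player's session on logout.
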(event `SpawnPlayer`
  (params (PlayerController :type "PlayerController Object Reference") (SelectedCharacter :type "Character Class Reference"))
  (bind _spawnpoints (`self.SpawnPoints`))
  (bind _returnvalue (`KismetArrayLibrary.Array_Length` _spawnpoints))
  (bind _outactors (`GameplayStatics.GetAllActorsOfClass` "/Script/Engine.PlayerStart"))
  (set `self.SpawnPoints` _outactors)
  (`KismetSystemLibrary.PrintString` (`KismetStringLibrary.Conv_IntToString` _returnvalue))
  (`/Engine/EditorBlueprintResources/StandardMacros.IsValid` (`Controller.K2_GetPawn` PlayerController)
    (:`Is Valid`
      (`KismetSystemLibrary.PrintString` "Es valido")
      (`self.K2_DestroyActor`))
    (:`Is Not Valid`
      _))
  (bind _returnvalue_2 (`|SpawnActorFromClass` SelectedCharacter (`self.GetTransform` (`|GetArrayItem` _spawnpoints (`KismetMathLibrary.RandomIntegerInRange` 0 (- _returnvalue 1)))) "AlwaysSpawn" "OverrideRootScale" null null))
  (`KismetSystemLibrary.PrintString` (`KismetSystemLibrary.GetDisplayName` _returnvalue_2))
  (`Controller.Possess` PlayerController _returnvalue_2))

(event `self.K2_OnSwapPlayerControllers`
  (params (OldPC :type "PlayerController Object Reference") (NewPC :type "PlayerController Object Reference"))
  (`KismetArrayLibrary.Array_Add` (`self.AllPlayerControllers`) NewPC))

(event `self.K2_OnLogout`
  (params (ExitingController :type "Controller Object Reference"))
  (bind _gameplaypc (message `/Game/_Blueprints/Gameplay/BPI_GameplayPC.GameplayPCref` ExitingController))
  (bind _gameinstance (message `/Game/_Blueprints/BPI_GameInstance.SteamGameInstanceRef` (`GameplayStatics.GetGameInstance`)))
  (message `/Game/_Blueprints/BPI_GameInstance.DestroySessionCaller` _gameinstance _gameplaypc))

(event `UpdateChat`
  (params (Sender :type Text) (ChatText :type Text))
  (for _array_element (`self.AllPlayerControllers`)
    (bind _gameplaypc (message `/Game/_Blueprints/Gameplay/BPI_GameplayPC.GameplayPCref` _array_element))
    (`/Game/_Blueprints/Gameplay/BP_GameplayPC.UpdateChatWindow` _gameplaypc Sender ChatText)))

(fn `GameplayGMRef`
  (returns (GameplayGMRef :type "/Game/_Blueprints/Gameplay/BP_GameplayGameMode Object Reference"))
  (return self))

(fn `UserConstructionScript`)