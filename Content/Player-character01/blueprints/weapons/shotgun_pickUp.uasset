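; Shotgun pickup actor that spins in the world until the player character collects it.
; Tick adds a fixed yaw step each frame to the skeletal mesh, so spin speed depends on frame rate.
; On overlap with ShotgunColision, it fills the first empty of the player's five item slots, sets Weapon2PickedUp and destroys itself.
; If every slot is occupied, the pickup stays in place.
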(event `self.ReceiveTick`
  (params (DeltaSeconds :type "Float (single-precision)"))
  (set `self.rota` (+ (`self.rota`) 1.0))
  (`SceneComponent.K2_SetWorldRotation` (`self.SkeletalMesh`) (`KismetMathLibrary.MakeRotator` 0.0 0.0 (`self.rota`)) false false))

(event `self.shotgunColision.OnComponentBeginOverlap`
  (params (OverlappedComponent :type "PrimitiveComponent Object Reference") (OtherActor :type "Actor Object Reference") (OtherComp :type "PrimitiveComponent Object Reference") (OtherBodyIndex :type Integer) (bFromSweep :type Boolean) (SweepResult :type "HitResult Structure (by ref)"))
  (bind _asplayer_character (cast `/Game/Player-character01/PlayerCharacter` OtherActor))
  (if (== (`/Game/Player-character01/PlayerCharacter.slot1item` _asplayer_character) 0)
    (set `/Game/Player-character01/PlayerCharacter.slot1item` 1 _asplayer_character)
    (set `/Game/Player-character01/PlayerCharacter.weapon2PickedUp` true _asplayer_character :!label _label)
    (`self.K2_DestroyActor`)
    (elif (== (`/Game/Player-character01/PlayerCharacter.slot2item` _asplayer_character) 0)
      (set `/Game/Player-character01/PlayerCharacter.slot2item` 1 _asplayer_character)
      (goto _label)
      (elif (== (`/Game/Player-character01/PlayerCharacter.slot3item` _asplayer_character) 0)
        (set `/Game/Player-character01/PlayerCharacter.slot3item` 1 _asplayer_character)
        (goto _label)
        (elif (== (`/Game/Player-character01/PlayerCharacter.slot4item` _asplayer_character) 0)
          (set `/Game/Player-character01/PlayerCharacter.slot4item` 1 _asplayer_character)
          (goto _label)
          (elif (== (`/Game/Player-character01/PlayerCharacter.slot5item` _asplayer_character) 0)
            (set `/Game/Player-character01/PlayerCharacter.slot5item` 1 _asplayer_character)
            (goto _label)))))))

(fn `UserConstructionScript`)