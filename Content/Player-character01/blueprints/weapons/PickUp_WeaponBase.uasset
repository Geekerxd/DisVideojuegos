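; PickUp_WeaponBase is a base weapon Blueprint that handles hitscan firing.
; SRV_FireWeapon spawns an attached muzzle flash and plays the fire sound, then line-traces on Visibility from the camera along its forward vector, ignoring itself and its owner.
; A hit receives point damage using the weapon's damage variables, with no instigator connected and the camera location passed as the hit direction.
; The graphs contain no pickup logic.
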(event `SRV_FireWeapon`
  (bind _camera (`self.Camera`))
  (`GameplayStatics.SpawnEmitterAttached` (`self.Muzzle flash`) (`self.SkeletalMesh`) "MuzzleFlash")
  (`GameplayStatics.PlaySoundAtLocation` (`self.weapon fire`) (`self.K2_GetActorLocation`) (struct) 1.0 1.0 0.0 null null null)
  (set `self.CameraLocation` (`SceneComponent.K2_GetComponentLocation` _camera))
  (set `self.CameraRotation` (`SceneComponent.K2_GetComponentRotation` _camera))
  (bind (_outhit _returnvalue) (`KismetSystemLibrary.LineTraceSingle` (`self.CameraLocation`) (+ (`self.CameraLocation`) (* (`KismetMathLibrary.GetForwardVector` (`self.CameraRotation`)) (`self.BulletDistance`))) "TraceTypeQuery1" true (`|MakeArray` (`self.GetOwner`) self :!type "Actor Object Reference")))
  (if _returnvalue
    (`GameplayStatics.ApplyPointDamage` (`.HitActor` (`GameplayStatics.BreakHitResult` _outhit)) (`self.WeaponDamage`) (`self.CameraLocation`) _outhit null null "/Script/Engine.DamageType")))

(fn `UserConstructionScript`
  (`parent.UserConstructionScript`))