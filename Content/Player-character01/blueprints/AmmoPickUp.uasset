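; AmmoPickUp is a world pickup that adds rifle ammo to the player when touched.
; On BeginPlay it spawns a glowing aura emitter and an attenuated fairy dust sound at its location, keeping references to both.
; Capsule overlap by a PlayerCharacter adds a fixed amount to TempRifle's ammo, destroys the actor, plays a pickup sound and removes the aura and ambient sound components.
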(event `self.ReceiveBeginPlay`
  (bind _returnvalue (`self.K2_GetActorLocation`))
  (bind _returnvalue_2 (`GameplayStatics.SpawnEmitterAtLocation` "/Game/Player-character01/aura/glowingAura.glowingAura" _returnvalue))
  (bind _returnvalue_3 (`GameplayStatics.SpawnSoundAtLocation` "/Game/Player-character01/aura/Fairy_Dust_Sound_Effect_Cue.Fairy_Dust_Sound_Effect_Cue" _returnvalue (struct) 1.0 1.0 0.0 "/Game/Player-character01/aura/dust.dust" null)))

(event `self.ReceiveTick`
  (params (DeltaSeconds :type "Float (single-precision)")))

(event `self.CapsuleAmmo.OnComponentBeginOverlap`
  (params (OverlappedComponent :type "PrimitiveComponent Object Reference") (OtherActor :type "Actor Object Reference") (OtherComp :type "PrimitiveComponent Object Reference") (OtherBodyIndex :type Integer) (bFromSweep :type Boolean) (SweepResult :type "HitResult Structure (by ref)"))
  (bind _asplayer_character (cast `/Game/Player-character01/PlayerCharacter` OtherActor))
  (bind _temprifle (`/Game/Player-character01/PlayerCharacter.TempRifle` _asplayer_character))
  (set `/Game/Player-character01/blueprints/weapons/weapon_Rifle.ammo` (+ (`/Game/Player-character01/blueprints/weapons/weapon_Rifle.ammo` _temprifle) 10) _temprifle)
  (`self.K2_DestroyActor`)
  (`GameplayStatics.SpawnSoundAtLocation` "/Game/MilitaryWeapSilver/Sound/Rifle/Cues/Rifle_AmmoPickup_Cue.Rifle_AmmoPickup_Cue" (`self.K2_GetActorLocation`) (struct) 1.0 1.0 0.0 null null)
  (`ActorComponent.K2_DestroyComponent` (stale `self.ReceiveBeginPlay` _returnvalue_2))
  (`ActorComponent.K2_DestroyComponent` (stale `self.ReceiveBeginPlay` _returnvalue_3)))

(fn `UserConstructionScript`)